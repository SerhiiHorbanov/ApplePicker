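; Apple tree actor that slides side to side along the Y axis and drops apples at a regular interval.
; Tick moves it by Speed and turns it back at the symmetric LeftAndRightEdge bounds.
; A looping timer randomly flips its direction based on ChanceToChangeDirection, while another spawns an Apple actor at the tree's transform every SecondsBetweenAppleDrops.
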(event `self.ReceiveBeginPlay`
  (`KismetSystemLibrary.K2_SetTimer` null "ChangeDirectionByChance" 0.1 true)
  (`KismetSystemLibrary.K2_SetTimer` null "DropApple" (`self.SecondsBetweenAppleDrops`) true))

(event `self.ReceiveTick`
  (params (DeltaSeconds :type "Float (single-precision)"))
  (bind _returnvalue (`KismetMathLibrary.Abs` (`self.Speed`)))
  (bind _y (.y (`self.K2_GetActorLocation`)))
  (if (> (* (`self.LeftAndRightEdge`) -1.0) _y)
    (set `self.Speed` _returnvalue))
  (if (> _y (`self.LeftAndRightEdge`))
    (set `self.Speed` (* _returnvalue -1.0)))
  (`self.K2_AddActorWorldOffset` (`KismetMathLibrary.MakeVector` 0.0 (* DeltaSeconds (`self.Speed`)))))

(fn `ChangeDirectionByChance`
  (if (< (`KismetMathLibrary.RandomFloat`) (`self.ChanceToChangeDirection`))
    (set `self.Speed` (* (`self.Speed`) -1.0))))

(fn `DropApple`
  (`|SpawnActorFromClass` "/Game/Blueprints/Apple.Apple_C" (`self.GetTransform`) "Undefined" "MultiplyWithRoot" null null))

(fn `UserConstructionScript`)