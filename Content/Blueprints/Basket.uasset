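; Basket is the catcher actor in an Apple Picker game, collecting apples and scoring them.
; On actor overlap it destroys any actor tagged "Apple", then increments Score on the ApplePickerGameState and prints the new total, or an error if the cast fails.
; A MoveTo function sets its location directly, without sweeping, for external code to reposition it.
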(event `self.ReceiveActorBeginOverlap`
  (params (OtherActor :type "Actor Object Reference"))
  (if (`self.ActorHasTag` OtherActor "Apple")
    (`self.K2_DestroyActor` OtherActor)
    (bind _asapple_picker_game_state (cast `/Game/ApplePickerGameState` (`GameplayStatics.GetGameState`))
      (:`then`
        (bind _result (`/Engine/EditorBlueprintResources/StandardMacros.IncrementInt` (`/Game/ApplePickerGameState.Score` _asapple_picker_game_state))
          (:`  `
            (bind _output_get (set `/Game/ApplePickerGameState.Score` _result _asapple_picker_game_state))
            (`KismetSystemLibrary.PrintString` (`KismetStringLibrary.Conv_IntToString` _output_get)))))
      (:`CastFailed`
        (`KismetSystemLibrary.PrintString` "GameState cast to ApplePickerGameState failed in Basket")))))

(event `self.Cube.OnComponentBeginOverlap`
  (params (OverlappedComponent :type "PrimitiveComponent Object Reference") (OtherActor :type "Actor Object Reference") (OtherComp :type "PrimitiveComponent Object Reference") (OtherBodyIndex :type Integer) (bFromSweep :type Boolean) (SweepResult :type "HitResult Structure (by ref)")))

(fn `MoveTo`
  (params (NewPosition :type "Vector Structure"))
  (`self.K2_SetActorLocation` NewPosition))

(fn `UserConstructionScript`)